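; Inventory that holds collectibles up to a size limit and tracks a current slot.
; Adding stores the actor's class with a placeholder "Test" tooltip in a struct array, then destroys the actor, so instance state is not kept.
; Removing returns the stored class and deletes that array entry, shifting later items down.
; Next and previous slot selection wraps around the inventory size, independent of item count.
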(fn AddCollectible
  (params (Collectible :type BP%20Collectible%20Object%20Reference))
  (bind _isinventoryfull (CallFunction|IsInventoryFull))
  (if _isinventoryfull
    (return false)
    (else
      (Utilities|Array|Add (Variables|Default|GetInventoryItems) (Utilities|Struct|MakeST_Collectible (Utilities|GetClass Collectible) "Test"))
      (Actor|DestroyActor Collectible)
      (return true))))

(fn IsInventoryFull
  (return (>= (Utilities|Array|Length (Variables|Default|GetInventoryItems)) (Variables|Default|GetInventorySize))))

(fn RemoveCollectible
  (params (InventorySlot :type Integer))
  (bind _inventoryitems (Variables|Default|GetInventoryItems))
  (bind _item (Utilities|Array|Get(acopy) _inventoryitems InventorySlot))
  (bind _collectible (Utilities|Struct|BreakST_Collectible _item))
  (if (Utilities|IsValidClass _collectible)
    (bind _output_get (LocalVariables|SetCollectible _collectible))
    (Utilities|Array|RemoveIndex (Variables|Default|GetInventoryItems) InventorySlot)
    (return true _output_get)
    (else
      (return false 0))))

(fn PreviousSlot
  (if (< (Math|Integer|%(Integer) (- (Variables|Default|GetcurrentInventorySlot) 1) (Variables|Default|GetInventorySize)) 0)
    (Variables|Default|SetcurrentInventorySlot (+ (Math|Integer|%(Integer) (- (Variables|Default|GetcurrentInventorySlot) 1) (Variables|Default|GetInventorySize)) (Variables|Default|GetInventorySize)))
    (else
      (Variables|Default|SetcurrentInventorySlot (Math|Integer|%(Integer) (- (Variables|Default|GetcurrentInventorySlot) 1) (Variables|Default|GetInventorySize)))))
  (return))

(fn NextSlot
  (Variables|Default|SetcurrentInventorySlot (Math|Integer|%(Integer) (+ (Variables|Default|GetcurrentInventorySlot) 1) (Variables|Default|GetInventorySize)))
  (return))

(fn GetCollectible
  (params (InventorySlot :type Integer))
  (bind _inventoryitems (Variables|Default|GetInventoryItems))
  (bind _item (Utilities|Array|Get(acopy) _inventoryitems InventorySlot))
  (bind (_collectible _tooltip) (Utilities|Struct|BreakST_Collectible _item))
  (return _collectible _tooltip))