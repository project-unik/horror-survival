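; BP_Usable_Actor is an interactable actor that detects when the player camera is looking at it from within range.
; Each Tick, if the camera is within RaycastLength, it line traces along the camera's forward vector against only its InteractableMesh component.
; The hit result drives both the mesh's custom depth rendering and the IsUsable flag, which are cleared when out of range.
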(event `self.ReceiveTick`
  (params (DeltaSeconds :type "Float (single-precision)"))
  (bind _returnvalue (`GameplayStatics.GetPlayerCameraManager` 0))
  (bind _raycastlength (`self.RaycastLength`))
  (bind _interactablemesh (`self.InteractableMesh`))
  (bind _transformcomponent (`PlayerCameraManager.TransformComponent` _returnvalue))
  (bind _returnvalue_2 (`SceneComponent.K2_GetComponentLocation` _transformcomponent))
  ;[1 1 1] If we are out of range, disable the render effect
  (if (<= (`self.GetDistanceTo` _returnvalue) _raycastlength)
    ;[1 1 1] Otherwise set the render effect if we look at the target
    (bind (_hitlocation _hitnormal _bonename _returnvalue_3) (`PrimitiveComponent.K2_LineTraceComponent` _interactablemesh _returnvalue_2 (+ _returnvalue_2 (* (`KismetMathLibrary.GetForwardVector` (`SceneComponent.K2_GetComponentRotation` _transformcomponent)) _raycastlength)) false false))
    (`PrimitiveComponent.SetRenderCustomDepth` _interactablemesh _returnvalue_3)
    (set `self.IsUsable` _returnvalue_3)
    (else
      (`PrimitiveComponent.SetRenderCustomDepth` _interactablemesh false)
      (set `self.IsUsable` false))))

(fn `UserConstructionScript`)