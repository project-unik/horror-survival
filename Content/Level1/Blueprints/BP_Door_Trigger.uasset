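; BP_Door_Trigger is a one-shot overlap trigger that unlocks and opens a linked BP_Interactable_Door.
; On the first overlap by any actor while WasTriggered is true, it clears that flag and casts the Door reference.
; It then unlocks the door, rotates it to its open yaw at the trigger's Speed and marks it open.
; A failed cast only prints an error, with the trigger already spent.
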(event `self.ReceiveActorBeginOverlap`
  (params (OtherActor :type "Actor Object Reference"))
  (if (`self.WasTriggered`)
    (set `self.WasTriggered` false)
    (bind _asbp_interactable_door (cast `/Game/Level1/Blueprints/BP_Interactable_Door` (`self.Door`))
      (:`then`
        (set `/Game/Level1/Blueprints/BP_Door.IsLocked` false _asbp_interactable_door)
        (`KismetSystemLibrary.PrintString` "Door was unlocked")
        (`/Game/Level1/Blueprints/BP_Door.SetDoorYaw` _asbp_interactable_door (`/Game/Level1/Blueprints/BP_Interactable_Door.YawWhenOpen` _asbp_interactable_door) (`self.Speed`) null)
        (set `/Game/Level1/Blueprints/BP_Door.IsOpen` true _asbp_interactable_door))
      (:`CastFailed`
        (`KismetSystemLibrary.PrintString` "This blueprint only works with Interactable_Door")))))

(fn `UserConstructionScript`)