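; BP_Blur_PP is a post process focus volume that drives a blur effect from player camera proximity and gaze.
; On BeginPlay it creates a dynamic instance of PP_Blur_M and assigns it to its PostProcess component as a blendable.
; Each tick, camera distance provides half the blend weight; a forward trace against BoxCollision adds centre-closeness, normalised by Y extent.
; That weight scales the BlurAmount parameter, which is zeroed out of range.
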(event `self.ReceiveBeginPlay`
  ;[1 1 1] Create post process settings and retrive reference to post process material in order to manipulate its shader parameters
  (bind _returnvalue (`KismetMaterialLibrary.CreateDynamicMaterialInstance` "/Game/Level1/Assets/Materials/PP_Blur_M.PP_Blur_M"))
  (set `self.BlurPPMaterial` _returnvalue)
  (set `PostProcessComponent.Settings` (make `PostProcessSettings` :`WeightedBlendables` (make `WeightedBlendables` (`|MakeArray` (make `WeightedBlendable` 1.0 _returnvalue)))) (`self.PostProcess`)))

(event `self.ReceiveTick`
  (params (DeltaSeconds :type "Float (single-precision)"))
  (bind _blurdistance (`self.BlurDistance`))
  (bind _blurppmaterial (`self.BlurPPMaterial`))
  (bind _returnvalue (`self.GetDistanceTo` (`GameplayStatics.GetPlayerCameraManager` 0) self))
  (bind _transformcomponent (`PlayerCameraManager.TransformComponent` (`GameplayStatics.GetPlayerCameraManager` 0)))
  (bind _postprocess (`self.PostProcess`))
  (bind _returnvalue_2 (`SceneComponent.K2_GetComponentLocation` _transformcomponent))
  (bind _returnvalue_3 (/ (- 1.0 (/ _returnvalue _blurdistance)) 2.0))
  ;[1 1 1] Calculate blur weight for post process focus volumes
  ;;[1 1 1] If we are out of range, just set the value to 0
  (if (<= _returnvalue _blurdistance)
    ;;[1 1 1] If we are in range, check if the player looks at this volume
    (bind (_hitlocation _hitnormal _bonename _returnvalue_4) (`PrimitiveComponent.K2_LineTraceComponent` (`self.BoxCollision`) _returnvalue_2 (+ _returnvalue_2 (* (`KismetMathLibrary.GetForwardVector` (`SceneComponent.K2_GetComponentRotation` _transformcomponent)) (`self.RaycastLength`))) true false))
    (if _returnvalue_4
      ;;[1 1 1] If we look at the current post process focus volume, we also take the difference between the raycast hit location and the centre  of the volume into account
      (bind _output_get (set `PostProcessComponent.BlendWeight` (`KismetMathLibrary.FClamp` (+ _returnvalue_3 (/ (- 1.0 (/ (`KismetMathLibrary.VSize` (- _hitlocation (`SceneComponent.K2_GetComponentLocation` _postprocess))) (.y (`.BoxExtent` (`self.GetActorBounds` self false))))) 2.0))) _postprocess))
      (`MaterialInstanceDynamic.SetScalarParameterValue` _blurppmaterial "BlurAmount" (* _output_get (`self.BlurImpactFactor`)))
      (else
        ;;[1 1 1] If we don't look at the current post process focus volume, we just take the position diff. into account
        (bind _output_get_2 (set `PostProcessComponent.BlendWeight` (`KismetMathLibrary.FClamp` _returnvalue_3) _postprocess))
        (`MaterialInstanceDynamic.SetScalarParameterValue` _blurppmaterial "BlurAmount" (* _output_get_2 (`self.BlurImpactFactor`))) ; Set the shader parameter
      ))
    (else
      (`MaterialInstanceDynamic.SetScalarParameterValue` (`self.BlurPPMaterial`) "BlurAmount" 0.0) ; Set the shader parameter
    )))

(fn `UserConstructionScript`)