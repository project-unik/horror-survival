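; Door actor that swings its Door component to a requested yaw at a given speed, with an optional sound at the door.
; SetDoorYaw treats a move to an equal or larger absolute yaw as opening, fires the rotation event, then stores the new yaw.
; The event plays or reverses the DoorRotation timeline, swapping old and new yaw when closing so one interpolation serves both directions.
; A ToggleVariable macro sets IsOpen opposite to its input.
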(event `DoorRot_Event`
  (params (NewYaw :type "Float (double-precision)") (OldYaw :type "Float (double-precision)") (Open :type Boolean) (Speed :type "Float (double-precision)") (Sound :type "SoundCue Object Reference"))
  (`TimelineComponent.SetPlayRate` (`self.DoorRotation`) Speed)
  (bind (_newthis _newother) (`self.Swap Float` NewYaw OldYaw (not Open))) ; NewYaw and OldYaw have to be swapped\ndepending on the door movement
  (`/Engine/EditorBlueprintResources/StandardMacros.IsValid` Sound
    (:`Is Valid`
      (`GameplayStatics.PlaySoundAtLocation` Sound (`SceneComponent.K2_GetComponentLocation` (`self.Door`))))
    (:`Is Not Valid`
      _))
  (if Open
    (bind (_direction _doorrotation) (`Timeline|DoorRotation` :!label _label)
      (:`Update`
        (`SceneComponent.K2_SetRelativeRotation` (`self.Door`) (`KismetMathLibrary.MakeRotator` 0.0 0.0 (+ (* _doorrotation (- _newthis _newother)) _newother)) false false)))
    (else
      (goto _label :!via `Reverse`))))

(fn `SetDoorYaw`
  (params (NewYaw :type "Float (double-precision)") (Speed :type "Float (double-precision)") (Sound :type "SoundCue Object Reference"))
  (bind _relativeyaw (`self.RelativeYaw`))
  (`self.DoorRot_Event` NewYaw _relativeyaw (>= (`KismetMathLibrary.Abs` NewYaw) (`KismetMathLibrary.Abs` _relativeyaw)) Speed Sound)
  (set `self.RelativeYaw` NewYaw))

(fn `Swap Float`
  (params (This :type "Float (double-precision)") (Other :type "Float (double-precision)") (Swap :type Boolean))
  (returns (NewThis :type "Float (double-precision)") (NewOther :type "Float (double-precision)"))
  (if Swap
    (return Other This)
    (else
      (return This Other))))

(fn `UserConstructionScript`)