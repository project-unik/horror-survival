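; Interactable door for Level1 that swings between open and closed yaw angles on the Interact input, or prints a message when locked.
; The press runs ToggleVariable, which flips IsOpen and branches on its previous value to call SetDoorYaw with the target angle and speed.
; The construction script initializes a usable child-actor component with the door mesh for outline rendering.
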(event `InputAction|Interact`
  (params (Key :type "Key Structure" :default "AnyKey"))
  ;[1 1 1] Door Interaction Logic
  (:`Pressed`
    (if (`self.IsLocked`)
      (`KismetSystemLibrary.PrintString` "Door is locked")
      (else
        (`self.ToggleVariable` (`self.IsOpen`)
          (:`WasTrue`
            (`self.SetDoorYaw` (`self.YawWhenClosed`) (`self.Speed`)) ; Door was Open so it needs to be closed to YawWhenClosed
          )
          (:`WasFalse`
            (`self.SetDoorYaw` (`self.YawWhenOpen`) (`self.Speed`)) ; See above
          ))))))

(fn `UserConstructionScript`
  ;[1 1 1] Initialize usable component to render outline
  (`/Game/Level1/Blueprints/BP_Utility_FL.InitializeUsableActorComponent` (`self.UsableChildActor`) (`self.Door`)))