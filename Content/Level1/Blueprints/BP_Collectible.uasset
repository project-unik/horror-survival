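; BP_Collectible is a collectible actor that the player character can pick up.
; Its construction script calls MakeUsable, which initializes a usable child actor component with the static mesh as its interactable mesh.
; The actor handles the Pickup input action itself, casting player 0's character to BP_Player_Character and passing itself to OnCollectorCollect.
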(event `InputAction|Pickup`
  (params (Key :type "Key Structure" :default "AnyKey"))
  (:`Pressed`
    (bind _asbp_player_character (cast `/Game/General/BP_Player_Character` (`GameplayStatics.GetPlayerCharacter` 0)))
    (`/Game/General/IF_Collector.OnCollectorCollect` _asbp_player_character self)))

(fn `MakeUsable`
  (returns (UsableChildActor :type "ChildActorComponent Object Reference"))
  (bind _usablechildactor (`self.UsableChildActor`))
  (`/Game/Level1/Blueprints/BP_Utility_FL.InitializeUsableActorComponent` _usablechildactor (`self.StaticMesh`))
  (return _usablechildactor))

(fn `UserConstructionScript`
  (`self.MakeUsable`))